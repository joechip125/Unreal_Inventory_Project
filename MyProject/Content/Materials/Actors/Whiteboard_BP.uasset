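; Whiteboard actor that can be drawn on at runtime by painting into a render target.
; BeginPlay creates the render target, assigns it to a dynamic board material with the texture parameter name left as None, and creates a marker material instance.
; DrawOnBoard passes a UV location to the marker material and draws it into the target.
; An unconnected line-trace snippet would supply that UV through FindCollisionUV.
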(event `self.ReceiveBeginPlay`
  (bind _whiteboard (`self.WhiteBoard`))
  (bind _returnvalue (`KismetRenderingLibrary.CreateRenderTarget2D` 2048 2048))
  (set `self.PaintBoardRT` _returnvalue)
  (bind _returnvalue_2 (`PrimitiveComponent.CreateDynamicMaterialInstance` _whiteboard 0 (`PrimitiveComponent.GetMaterial` _whiteboard 0) "None"))
  (`MaterialInstanceDynamic.SetTextureParameterValue` _returnvalue_2 "None" (`self.PaintBoardRT`))
  (`PrimitiveComponent.SetMaterial` (`self.WhiteBoard`) 0 _returnvalue_2)
  (bind _returnvalue_3 (`KismetMaterialLibrary.CreateDynamicMaterialInstance` "/Game/Materials/M_Marker.M_Marker"))
  (set `self.MarkerMID` _returnvalue_3))

(event `DrawOnBoard`
  (params (DrawLocation :type "Vector2D Structure"))
  (`MaterialInstanceDynamic.SetVectorParameterValue` (`self.MarkerMID`) "DrawLocation" (`KismetMathLibrary.Conv_VectorToLinearColor` (`KismetMathLibrary.Conv_Vector2DToVector` DrawLocation 0.1)))
  (`KismetRenderingLibrary.DrawMaterialToRenderTarget` (`self.PaintBoardRT`) (`self.MarkerMID`)))

(fn `UserConstructionScript`)
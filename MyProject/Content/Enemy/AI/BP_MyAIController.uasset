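; Enemy AI controller that runs the GP_BehaviourTree behavior tree at BeginPlay.
; Its AIPerception component writes each updated actor to the TargetPlayer blackboard key, without checking actor type or whether sensing succeeded.
; An uncalled SetAndForget graph would set that key to the player character, then clear it after a short delay.
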(event `self.ReceiveBeginPlay`
  (`self.RunBehaviorTree` "/Game/Enemy/AI/GP_BehaviourTree.GP_BehaviourTree"))

(event `self.AIPerception.OnTargetPerceptionUpdated`
  (params (Actor :type "Actor Object Reference") (Stimulus :type "AIStimulus Structure"))
  (`BlackboardComponent.SetValueAsObject` (`AIBlueprintHelperLibrary.GetBlackboard` null) "TargetPlayer" Actor))

(fn `UserConstructionScript`)
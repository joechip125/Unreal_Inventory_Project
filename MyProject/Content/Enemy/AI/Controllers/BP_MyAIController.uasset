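; AI controller that runs the MoveBoxesTree behavior tree on BeginPlay and feeds it perception results through the blackboard.
; A sensed stimulus stores the actor as TargetActor, while a lost one stores the stimulus location as TargetDestination.
; Each perception update also calls SetBaseState to switch a base-state enum, but that function writes to a blackboard key named None.
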(event `self.ReceiveBeginPlay`
  (`self.RunBehaviorTree` "/Game/Enemy/AI/Trees/MoveBoxesTree.MoveBoxesTree"))

(event `self.AIPerception.OnTargetPerceptionUpdated`
  (params (Actor :type "Actor Object Reference") (Stimulus :type "AIStimulus Structure"))
  (if Stimulus_bSuccessfullySensed
    (`BlackboardComponent.SetValueAsObject` (`AIBlueprintHelperLibrary.GetBlackboard` null) "TargetActor" Actor)
    (`self.SetBaseState` "NewEnumerator1")
    (else
      (`BlackboardComponent.SetValueAsVector` (`AIBlueprintHelperLibrary.GetBlackboard` null) "TargetDestination" Stimulus_StimulusLocation)
      (`self.SetBaseState` "NewEnumerator2"))))

(fn `SetBaseState`
  (params (NewState :type "/Game/Enemy/AI/Enums/BaseState Enum" :default "NewEnumerator0"))
  (`BlackboardComponent.SetValueAsEnum` (`AIBlueprintHelperLibrary.GetBlackboard` null) "None" (enumliteral `/Game/Enemy/AI/Enums/BaseState` NewState)))

(fn `UserConstructionScript`)
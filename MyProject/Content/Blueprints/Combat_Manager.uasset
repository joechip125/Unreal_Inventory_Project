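; Combat manager component that detects weapon hits from a HitTrace socket on its owner's equipped object component.
; TraceForHit sweeps a debug-drawn box trace on the Visibility channel from the stored socket location to the current one, covering movement between samples.
; Each hit actor joins an ignore list to prevent repeat hits and is broadcast through OnHit.
; Separate functions refresh the stored location and clear the list.
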(fn `GetCurrentSocketLocation`
  (returns (Location :type "Vector Structure"))
  (return (`SceneComponent.GetSocketLocation` (`Actor.GetComponentByClass` (`self.GetOwner`) "/Game/Inventory/Equipment/EquippedObjectComponent.EquippedObjectComponent_C") "HitTrace")))

(fn `ResetActorsToIgnore`
  (`KismetArrayLibrary.Array_Clear` (`self.Actors to Ignore`)))

(fn `TraceForHit`
  (bind (_outhit _returnvalue) (`KismetSystemLibrary.BoxTraceSingle` (`self.LastSocketLocation`) (`self.GetCurrentSocketLocation`) (10.0 10.0 10.0) (struct) "TraceTypeQuery1" true (`self.Actors to Ignore`) "ForDuration"))
  (if _returnvalue
    (`KismetArrayLibrary.Array_AddUnique` (`self.Actors to Ignore`) (`.HitActor` (`GameplayStatics.BreakHitResult` _outhit)))
    (`self.OnHit` _outhit)))

(fn `UpdateLastSocketLocation`
  (set `self.LastSocketLocation` (`self.GetCurrentSocketLocation`)))